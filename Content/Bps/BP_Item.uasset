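; BP_Item is a collectible pickup that triggers when BP_ThirdPersonCharacter overlaps its Rango component.
; It increments the character's item count and refreshes the counter in that character's game UI.
; It then opens a WBP_Algoritmo widget, shows the mouse cursor, pauses the game, calls the widget's Pantalla function and destroys itself.
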(event OnComponentBeginOverlap(Rango)
  (params (OverlappedComponent :type Primitive%20Component%20Object%20Reference) (OtherActor :type Actor%20Object%20Reference) (OtherComp :type Primitive%20Component%20Object%20Reference) (OtherBodyIndex :type Integer) (bFromSweep :type Boolean) (SweepResult :type Hit%20Result%20Structure%20%28by%20ref%29))
  (bind _asbp_third_person_character (Utilities|Casting|CastToBP_ThirdPersonCharacter OtherActor))
  (Variables|/Game/ThirdPerson/Blueprints/BP_ThirdPersonCharacter.BP_ThirdPersonCharacter_C|SetItems _asbp_third_person_character (+ (Variables|/Game/ThirdPerson/Blueprints/BP_ThirdPersonCharacter.BP_ThirdPersonCharacter_C|GetItems _asbp_third_person_character) 1))
  (Default|ContItems (Variables|/Game/ThirdPerson/Blueprints/BP_ThirdPersonCharacter.BP_ThirdPersonCharacter_C|GetUIJuego _asbp_third_person_character))
  (bind _returnvalue (UserInterface|CreateWidget "/Game/Widget/WBP_Algoritmo.WBP_Algoritmo_C"))
  (UserInterface|Viewport|AddtoPlayerScreen _returnvalue)
  (Variables|/Script/Engine.PlayerController|SetbShowMouseCursor (Game|GetPlayerController 0) true)
  (Game|SetGamePaused true)
  (Default|Pantalla _returnvalue)
  (Actor|DestroyActor))

(fn ConstructionScript)